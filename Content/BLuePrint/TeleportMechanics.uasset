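; Teleporter actor that sends anything overlapping its Capsule to the Sphere's location and rotation.
; The construction script places the Sphere from the TeleportLocation transform; for the player, teleporting also aligns control rotation and zeroes velocity.
; A Box reports overlap begin and end to actors implementing BPI_ChrachterAttachment, with debug prints on entry.
; A holding-status event sets ObectPickUp, which suppresses the end-overlap message while true.
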(event `self.Capsule.OnComponentBeginOverlap`
  (params (OverlappedComponent :type "PrimitiveComponent Object Reference") (OtherActor :type "Actor Object Reference") (OtherComp :type "PrimitiveComponent Object Reference") (OtherBodyIndex :type Integer) (bFromSweep :type Boolean) (SweepResult :type "HitResult Structure (by ref)"))
  (bind _returnvalue (`GameplayStatics.GetPlayerCharacter` 0))
  (bind (_returnvalue_location _returnvalue_rotation) (`KismetMathLibrary.BreakTransform` (`SceneComponent.K2_GetComponentToWorld` (`self.Sphere`))))
  ; teleport
  (`SceneComponent.K2_SetWorldTransform` (`Actor.RootComponent` OtherActor) (`KismetMathLibrary.MakeTransform` _returnvalue_location _returnvalue_rotation) false false)
  (if (== OtherActor _returnvalue)
    (`Controller.SetControlRotation` (`GameplayStatics.GetPlayerController` 0) (`self.K2_GetActorRotation` _returnvalue))
    (set `MovementComponent.Velocity` (0.0 0.0 0.0) (`Character.CharacterMovement` _returnvalue))))

(event `self.Box.OnComponentBeginOverlap`
  (params (OverlappedComponent :type "PrimitiveComponent Object Reference") (OtherActor :type "Actor Object Reference") (OtherComp :type "PrimitiveComponent Object Reference") (OtherBodyIndex :type Integer) (bFromSweep :type Boolean) (SweepResult :type "HitResult Structure (by ref)"))
  (`KismetSystemLibrary.PrintString` (`KismetSystemLibrary.GetDisplayName` OtherActor))
  (if (`KismetSystemLibrary.DoesImplementInterface` OtherActor "/Game/BLuePrint/BPI_ChrachterAttachment.BPI_ChrachterAttachment_C")
    (message `/Game/BLuePrint/BPI_ChrachterAttachment.OverlapStatusChange` OtherActor "NewEnumerator0" null)
    (`KismetSystemLibrary.PrintString` "overlaping")))

(event `self.Box.OnComponentEndOverlap`
  (params (OverlappedComponent :type "PrimitiveComponent Object Reference") (OtherActor :type "Actor Object Reference") (OtherComp :type "PrimitiveComponent Object Reference") (OtherBodyIndex :type Integer))
  (if (and (`KismetSystemLibrary.DoesImplementInterface` OtherActor "/Game/BLuePrint/BPI_ChrachterAttachment.BPI_ChrachterAttachment_C") (not (`self.ObectPickUp`)))
    (message `/Game/BLuePrint/BPI_ChrachterAttachment.OverlapStatusChange` OtherActor "NewEnumerator1" null)))

(event `/Game/BLuePrint/BPI_ObjectAttachment.ChangeHoldingStatusOnObject`
  (params (isHolding :type Boolean))
  (set `self.ObectPickUp` isHolding))

(fn `UserConstructionScript`
  (`SceneComponent.K2_SetRelativeTransform` (`self.Sphere`) (`self.Teleport Location`) false false))