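; PickUpPortal is a pickup actor that tells overlapping characters when it is available to pick up.
; Its Box overlap events send a status through BPI_ChrachterAttachment, passing itself as the pickup actor on begin overlap.
; ChangeHoldingStatusonObject sets ObectPickUp, which suppresses the end-overlap message while the object is held.
; Begin overlap also prints debug strings.
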(event `self.Box.OnComponentBeginOverlap`
  (params (OverlappedComponent :type "PrimitiveComponent Object Reference") (OtherActor :type "Actor Object Reference") (OtherComp :type "PrimitiveComponent Object Reference") (OtherBodyIndex :type Integer) (bFromSweep :type Boolean) (SweepResult :type "HitResult Structure (by ref)"))
  (`KismetSystemLibrary.PrintString` (`KismetSystemLibrary.GetDisplayName` OtherActor))
  (if (`KismetSystemLibrary.DoesImplementInterface` OtherActor "/Game/BLuePrint/BPI_ChrachterAttachment.BPI_ChrachterAttachment_C")
    (message `/Game/BLuePrint/BPI_ChrachterAttachment.OverlapStatusChange` OtherActor "NewEnumerator0" self)
    (`KismetSystemLibrary.PrintString` "overlaping")))

(event `self.Box.OnComponentEndOverlap`
  (params (OverlappedComponent :type "PrimitiveComponent Object Reference") (OtherActor :type "Actor Object Reference") (OtherComp :type "PrimitiveComponent Object Reference") (OtherBodyIndex :type Integer))
  (if (and (`KismetSystemLibrary.DoesImplementInterface` OtherActor "/Game/BLuePrint/BPI_ChrachterAttachment.BPI_ChrachterAttachment_C") (not (`self.ObectPickUp`)))
    (message `/Game/BLuePrint/BPI_ChrachterAttachment.OverlapStatusChange` OtherActor "NewEnumerator1" null)))

(event `/Game/BLuePrint/BPI_ObjectAttachment.ChangeHoldingStatusOnObject`
  (params (isHolding :type Boolean))
  (set `self.ObectPickUp` isHolding))

(fn `UserConstructionScript`)